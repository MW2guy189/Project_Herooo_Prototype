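; BPC_Attack_System is a combat component for sword attack combos, currently holding a single attack step.
; The swordattack event buffers a request while attacking or dispatches on AttackIndex to Attack1, which plays a montage behind a DoOnce and advances the index.
; The combo event replays any buffered request through that dispatch, and stopcombo resets the state.
; The IA_Attack input checks CanAttack but triggers nothing yet.
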(event `Attack 1`
  ;[1 1 1] attack 1
  (`/Engine/EditorBlueprintResources/StandardMacros.DoOnce` false :!label _label
    (:`Completed`
      (`KismetSystemLibrary.Delay` 0.1)
      (`|PlayMontage` null
        (:`then`
          (set `self.attack index` 1)
          (goto _label :!via `Reset`))))))

(event `EnhancedInput|/Game/ThirdPerson/Input/Actions/IA_Attack`
  (params (ActionValue :type Boolean) (ElapsedSeconds :type "Float (double-precision)") (TriggeredSeconds :type "Float (double-precision)") (InputAction :type "InputAction Object Reference" :default "/Game/ThirdPerson/Input/Actions/IA_Attack.IA_Attack"))
  ;[1 1 1] attack input
  (:`Started`
    (if (`self.can attack?`)
      _)))

(event `sword attack`
  ;[1 1 1] Sword Attack
  (if (`self.is attacking?`)
    (set `self.save attack?` true)
    (else
      (set `self.save attack?` false)
      (switch `int` (`self.attack index`) :!label _label_2
        (:`0`
          (`self.Attack 1`))))))

(event `sword attack combo`
  ;[1 1 1] Combo Continue
  (if (`self.save attack?`)
    (set `self.save attack?` false)
    (goto _label_2)))

(event `stop combo`
  ;[1 1 1] Stop Combo / Attack
  (set `self.is attacking?` false)
  (set `self.attack index` 0))