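; BP_Dummy is a stealth-assassination victim that shows a prompt widget while the third-person character overlaps its sphere.
; Every tick the widget rotates to face the player camera.
; StealthBackAssassination plays the paired knife victim montage, hides the prompt and returns a reference location and the actor's rotation to the caller.
; It also triggers the Ragdoll event, which uses delays to play a death sound and then enable mesh physics.
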(event `self.ReceiveTick`
  (params (DeltaSeconds :type "Float (single-precision)"))
  (`SceneComponent.K2_SetWorldRotation` (`self.AssassinatePrompt_Widget`) (`KismetMathLibrary.FindLookAtRotation` (`SceneComponent.K2_GetComponentLocation` (`self.AssassinatePrompt_Widget`)) (`SceneComponent.K2_GetComponentLocation` (`PlayerCameraManager.TransformComponent` (`GameplayStatics.GetPlayerCameraManager` 0)))) false false))

(event `Ragdoll`
  ;[1 1 1] Ragdoll
  (`|ExecutionSequence`
    (:`then_0`
      (`KismetSystemLibrary.Delay` 2.0)
      (`PrimitiveComponent.SetSimulatePhysics` (`self.Mesh`) true))
    (:`then_1`
      (`KismetSystemLibrary.Delay` 1.7)
      (`GameplayStatics.PlaySoundAtLocation` "/Game/RPGSeries/SFX/SC_Death.SC_Death" (`self.K2_GetActorLocation`) (struct) 1.0 1.0 0.0 null null null null))))

(event `self.Sphere.OnComponentBeginOverlap`
  (params (OverlappedComponent :type "PrimitiveComponent Object Reference") (OtherActor :type "Actor Object Reference") (OtherComp :type "PrimitiveComponent Object Reference") (OtherBodyIndex :type Integer) (bFromSweep :type Boolean) (SweepResult :type "HitResult Structure (by ref)"))
  ;[1 1 1] assassinate prompt
  (cast `/Game/ThirdPerson/Blueprints/BP_ThirdPersonCharacter` OtherActor)
  (`SceneComponent.SetVisibility` (`self.AssassinatePrompt_Widget`) true false))

(event `self.Sphere.OnComponentEndOverlap`
  (params (OverlappedComponent :type "PrimitiveComponent Object Reference") (OtherActor :type "Actor Object Reference") (OtherComp :type "PrimitiveComponent Object Reference") (OtherBodyIndex :type Integer))
  ;[1 1 1] assassinate prompt
  (cast `/Game/ThirdPerson/Blueprints/BP_ThirdPersonCharacter` OtherActor)
  (`SceneComponent.SetVisibility` (`self.AssassinatePrompt_Widget`) false false))

(fn `StealthBackAssassination`
  (returns (RefLocation :type "Vector Structure") (AssassinationRotation :type "Rotator Structure"))
  (`self.PlayAnimMontage` "/Game/RPGSeries/Assassination/Paired_Knife_Stealth_KidneyAndNeck_Vic_Montage.Paired_Knife_Stealth_KidneyAndNeck_Vic_Montage")
  (`self.Ragdoll`)
  (`SceneComponent.SetVisibility` (`self.AssassinatePrompt_Widget`) false false)
  (return (`SceneComponent.K2_GetComponentLocation` (`self.assssinref`)) (`self.K2_GetActorRotation`)))

(fn `UserConstructionScript`)